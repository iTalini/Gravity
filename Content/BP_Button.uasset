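; BP_Button is a pressable button actor that reacts to the player character's press input.
; Each Tick, while it can be pressed, it polls the WasPress flag on the player's BP_MyChar.
; When that flag is set, it clears it, disables further presses and plays Timeline_ChangeButton, forwarding the track value to TimelineProgress and calling TimelineFinish at the end.
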(event EventBeginPlay)

(event Collision|EventActorBeginOverlap
  (params (OtherActor :type Actor%20Object%20Reference)))

(event EventTick
  (params (DeltaSeconds :type Float%20%28single-precision%29))
  (bind _returnvalue (Class|ParentButton|GetCanPress))
  (if _returnvalue
    (bind _asbp_my_char (Utilities|Casting|CastToBP_MyChar (Game|Player|GetPlayerPawn 0)))
    (bind _returnvalue_2 (Class|MyCharacter|GetWasPress _asbp_my_char))
    (if _returnvalue_2
      (Utilities|Set|WasPress _asbp_my_char false)
      (Utilities|Set|CanPress false)
      (bind _newtrack_0 (Timeline|Timeline_ChangeButton Play)
        (:Update
          (Class|ParentButton|TimelineProgress _newtrack_0))
        (:Finished
          (Class|ParentButton|TimelineFinish))))))

(fn ConstructionScript)